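; Behavior tree task that moves an adult AI pawn relative to its blackboard Target, using a style picked by ComportementIndex.
; It either heads to the target's location, leads a BP_Monkey 400 units along its velocity, or overshoots that predicted point by the pawn's offset to it.
; The task reports success regardless of move result, and only the direct move wires the Pawn input of AIMoveTo.
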(event EventReceiveExecuteAI
  (params (OwnerController :type AI%20Controller%20Object%20Reference) (ControlledPawn :type Pawn%20Object%20Reference))
  (bind _target (Variables|Default|GetTarget))
  (bind _target_2 (Variables|Default|GetTarget))
  (bind _returnvalue (Class|BTFunctionLibrary|GetBlackboardValueasObject _target))
  (bind _returnvalue_2 (Class|BTFunctionLibrary|GetBlackboardValueasObject _target_2))
  (bind _asbp_monkey (Utilities|Casting|CastToBP_Monkey _returnvalue))
  (bind _asbp_monkey_2 (Utilities|Casting|CastToBP_Monkey _returnvalue_2))
  (bind _returnvalue_3 (Transformation|GetActorLocation _asbp_monkey))
  (bind _returnvalue_4 (Transformation|GetVelocity _asbp_monkey))
  (bind _returnvalue_5 (Math|Vector|Normalize _returnvalue_4))
  (bind _returnvalue_6 (* _returnvalue_5 4e+02))
  (bind _returnvalue_7 (+ _returnvalue_3 _returnvalue_6))
  (switch int (Class|BTFunctionLibrary|GetBlackboardValueasInt (Variables|Default|GetComportementIndex))
    (:0
      (AI|AIMoveTo ControlledPawn (Transformation|GetActorLocation (.AsActor (Utilities|Casting|CastToActor (Class|BTFunctionLibrary|GetBlackboardValueasObject (Variables|Default|GetTarget))))) 0 5.0 false
        (:then
          _)
        (:OnSuccess
          _)
        (:OnFail
          _))
      (AI|BehaviorTree|FinishExecute true))
    (:1
      (AI|AIMoveTo 0 (+ (Transformation|GetActorLocation _asbp_monkey_2) (* (Math|Vector|Normalize (Variables|/Script/Engine.MovementComponent|GetVelocity (Variables|/Script/Engine.Character|GetCharacterMovement _asbp_monkey_2))) 4e+02)) 0 5.0 false
        (:then
          _)
        (:OnSuccess
          _)
        (:OnFail
          _))
      (AI|BehaviorTree|FinishExecute true))
    (:2
      (AI|AIMoveTo 0 (+ (- _returnvalue_7 (Transformation|GetActorLocation ControlledPawn)) _returnvalue_7) 0 5.0 false
        (:then
          _)
        (:OnSuccess
          _)
        (:OnFail
          _))
      (AI|BehaviorTree|FinishExecute true))))