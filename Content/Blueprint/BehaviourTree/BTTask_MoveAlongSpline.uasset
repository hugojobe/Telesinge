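; Behaviour tree task that advances a BP_EnemyParent pawn along the spline stored in the blackboard.
; Each execution adds max walk speed times four frame deltas to SplineDistance, then writes the DistanceOnSpline vector and issues AIMoveTo to that spline point.
; It finishes successfully without waiting for the move.
; At the spline's end it instead calls OnEndOfSplineReachedMessage on the enemy, without finishing the task.
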(event EventReceiveExecuteAI
  (params (OwnerController :type AI%20Controller%20Object%20Reference) (ControlledPawn :type Pawn%20Object%20Reference))
  (bind (_x _y _z) (Math|Vector|BreakVector "0, 0, 0"))
  (bind _spline (Variables|Default|GetSpline))
  (bind _returnvalue (Class|BTFunctionLibrary|GetBlackboardValueasObject _spline))
  (bind _asspline_component (Utilities|Casting|CastToSplineComponent _returnvalue))
  (bind _output_get (Variables|Default|SetEnemy%20Parent (.AsBP%20Enemy%20Parent (Utilities|Casting|CastToBP_EnemyParent ControlledPawn))))
  (if (>= (+ (* (Variables|/Script/Engine.CharacterMovementComponent|GetMaxWalkSpeed (Variables|/Script/Engine.Character|GetCharacterMovement _output_get)) (* (Utilities|Time|GetWorldDeltaSeconds) 4.0)) (Class|BTFunctionLibrary|GetBlackboardValueasFloat (Variables|Default|GetSplineDistance))) (Spline|GetSplineLength _asspline_component))
    (Class|BPINPC|OnEndOfSplineReached(Message) (Variables|Default|GetEnemy%20Parent))
    (else
      (Class|BTFunctionLibrary|SetBlackboardValueasFloat (Variables|Default|GetSplineDistance) (+ (* (Variables|/Script/Engine.CharacterMovementComponent|GetMaxWalkSpeed (Variables|/Script/Engine.Character|GetCharacterMovement _output_get)) (* (Utilities|Time|GetWorldDeltaSeconds) 4.0)) (Class|BTFunctionLibrary|GetBlackboardValueasFloat (Variables|Default|GetSplineDistance))))
      (AI|BehaviorTree|SetBlackboardValueasVector (Variables|Default|GetDistanceOnSpline) (Math|Vector|MakeVector _x _y (+ _z (Variables|/Script/Engine.CapsuleComponent|GetCapsuleHalfHeight (Variables|/Script/Engine.Character|GetCapsuleComponent (Variables|Default|GetEnemy%20Parent))))))
      (AI|AIMoveTo (Variables|Default|GetEnemy%20Parent) (.location (Spline|GetTransformatDistanceAlongSpline _asspline_component (+ (* (Variables|/Script/Engine.CharacterMovementComponent|GetMaxWalkSpeed (Variables|/Script/Engine.Character|GetCharacterMovement _output_get)) (* (Utilities|Time|GetWorldDeltaSeconds) 4.0)) (Class|BTFunctionLibrary|GetBlackboardValueasFloat (Variables|Default|GetSplineDistance))) "World" false)) 0 1.0 false
        (:then
          _)
        (:OnSuccess
          _)
        (:OnFail
          _))
      (AI|BehaviorTree|FinishExecute true))))