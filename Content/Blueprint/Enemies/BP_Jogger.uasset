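; Jogger enemy with male or female animations and sounds, playing idle sounds at random intervals and destroying itself and its item at spline end.
; When stolen from, it halts, turns to the monkey, plays a reaction montage, then chases it through AI blackboard keys.
; When close, it plays an attack montage, clears the chase target and briefly pauses movement.
; Theft and proximity events extend parent class logic.
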(event Custom|MakePause
  (Audio|PlaySoundatLocation (select (Variables|Default|GetcharGenre) "/Game/Sound/PNJPark/PNJ_Femme/IDDLE/SC_FemmeIddle.SC_FemmeIddle" "/Game/Sound/PNJPark/Joggeur/Iddle/SC_JoggeurIddle.SC_JoggeurIddle") (Transformation|GetActorLocation) "0, 0, 0" 1.0 1.0 0.0 0 0 0 0)
  (Utilities|FlowControl|Delay (Math|Random|RandomFloatinRange 2.0 4.5))
  (Utilities|Time|SetTimerbyEvent (delegate Custom|MakePause) (Math|Random|RandomFloatinRange 5.0 15.0)))

(event EventOnceStealed
  (bind _returnvalue (Transformation|GetActorLocation))
  (bind _self self)
  (bind _monkey (Variables|Default|GetMonkey))
  (bind _returnvalue_2 (AI|GetAIController _self))
  (bind _returnvalue_3 (Transformation|GetActorLocation _monkey))
  (bind _returnvalue_4 (AI|GetBlackboard _returnvalue_2))
  (|CallParentFunction)
  (AI|Components|Blackboard|SetValueasBool (AI|GetBlackboard (AI|GetAIController self)) (Utilities|Name|MakeLiteralName "CanMove") false)
  (Variables|/Script/Engine.CharacterMovementComponent|SetbOrientRotationToMovement (Variables|Character|GetCharacterMovement) false)
  (Transformation|SetActorRotation (Math|Rotator|FindLookatRotation (Math|Vector|MakeVector (.x _returnvalue) (.y _returnvalue) 0.0) (Math|Vector|MakeVector (.x _returnvalue_3) (.y _returnvalue_3) 0.0)))
  (bind _returnvalue_5 (Animation|Montage|MontagePlay (Components|SkeletalMesh|GetAnimInstance (Variables|Character|GetMesh)) "/Game/Mesh/NPCs/Anims/Reaction_Montage.Reaction_Montage" 1.0 "MontageLength" 0.0 true))
  (Audio|PlaySoundatLocation (select (Variables|Default|GetcharGenre) "/Game/Sound/PNJPark/PNJ_Femme/Interaction/SC_FEMMEinteraction.SC_FEMMEinteraction" "/Game/Sound/PNJPark/Joggeur/Interaction/sc_JoggeurInteraction.sc_JoggeurInteraction") (Transformation|GetActorLocation) "0, 0, 0" 1.0 1.0 0.0 0 0 0 0)
  (Utilities|FlowControl|Delay _returnvalue_5)
  (Variables|Default|SetCanCatchMonkey true)
  (Variables|/Script/Engine.CharacterMovementComponent|SetbOrientRotationToMovement (Variables|Character|GetCharacterMovement) true)
  (AI|Components|Blackboard|SetValueasObject _returnvalue_4 (Utilities|Name|MakeLiteralName "RunTarget") (Variables|Default|GetMonkey))
  (AI|Components|Blackboard|SetValueasBool _returnvalue_4 (Utilities|Name|MakeLiteralName "IsReadyToFollowSpline") false)
  (AI|Components|Blackboard|SetValueasBool (AI|GetBlackboard (AI|GetAIController self)) (Utilities|Name|MakeLiteralName "CanMove") true))

(event EventOnEndOfSplineReached
  (bind _iteminstance (Variables|Default|GetItemInstance))
  (Utilities|IsValid _iteminstance
    (:Is%20Valid
      (Actor|DestroyActor _iteminstance))
    (:Is%20Not%20Valid
      _))
  (Actor|DestroyActor))

(event EventOnceClosetoMonkey
  (|CallParentFunction)
  ;[1 0 0] Attaque
  (Audio|PlaySoundatLocation (select (Variables|Default|GetcharGenre) "/Game/Sound/PNJPark/PNJ_Femme/attack/SC_FemmeAttaque.SC_FemmeAttaque" "/Game/Sound/PNJPark/PNJ_homme/SC_Hommeattack.SC_Hommeattack") (Transformation|GetActorLocation) "0, 0, 0" 1.0 1.0 0.0 0 0 0 0)
  (Animation|Montage|MontagePlay (Components|SkeletalMesh|GetAnimInstance (Variables|Character|GetMesh)) "/Game/Mesh/NPCs/Anims/huge_attack_Montage.huge_attack_Montage" 1.0 "MontageLength" 0.0 true)
  (Utilities|FlowControl|Delay 1.5)
  (AI|Components|Blackboard|ClearValue (AI|GetBlackboard (AI|GetAIController self)) (Utilities|Name|MakeLiteralName "RunTarget"))
  (Variables|Default|SetCanCatchMonkey false)
  (AI|Components|Blackboard|SetValueasBool (AI|GetBlackboard (AI|GetAIController self)) (Utilities|Name|MakeLiteralName "CanMove") false)
  (Utilities|FlowControl|Delay 0.5)
  (AI|Components|Blackboard|SetValueasBool (AI|GetBlackboard (AI|GetAIController self)) (Utilities|Name|MakeLiteralName "CanMove") true))

(event EventBeginPlay
  (|CallParentFunction)
  (Class|SkeletalMeshComponent|SetAnimClass (Variables|Character|GetMesh) (select (Variables|Default|GetcharGenre) "/Game/Blueprint/AnimBlueprint/ABP_JoggerF.ABP_JoggerF_C" "/Game/Blueprint/AnimBlueprint/ABP_Jogger.ABP_Jogger_C"))
  (Utilities|Time|SetTimerbyEvent (delegate Custom|MakePause) (Math|Random|RandomFloatinRange 5.0 15.0)))

(fn ConstructionScript
  (|CallParentFunction))

(fn GetPatrolRoute
  (return 0))