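; BP_Papy is an enemy character that pauses at random intervals and destroys itself and its item upon reaching the end of its spline.
; A self-rescheduling timer toggles the AI blackboard's CanMove flag to create the pauses.
; When stolen from, it halts, turns toward the Monkey and plays a 360 attack montage while a timeline drives slash material parameters, then resumes moving.
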(event Custom|MakePause
  (AI|Components|Blackboard|SetValueasBool (AI|GetBlackboard (AI|GetAIController self)) (Utilities|Name|MakeLiteralName "CanMove") false)
  (Utilities|FlowControl|Delay (Math|Random|RandomFloatinRange 2.0 4.5))
  (AI|Components|Blackboard|SetValueasBool (AI|GetBlackboard (AI|GetAIController self)) (Utilities|Name|MakeLiteralName "CanMove") true)
  (Utilities|Time|SetTimerbyEvent (delegate Custom|MakePause) (Math|Random|RandomFloatinRange 5.0 15.0)))

(event EventOnceStealed
  (bind _returnvalue (Transformation|GetActorLocation))
  (bind _monkey (Variables|Default|GetMonkey))
  (bind _slash02 (Variables|Default|GetSlash02))
  (bind _returnvalue_2 (Transformation|GetActorLocation _monkey))
  (|CallParentFunction)
  (Variables|/Script/Engine.CharacterMovementComponent|SetbOrientRotationToMovement (Variables|Character|GetCharacterMovement) false)
  (Transformation|SetActorRotation (Math|Rotator|FindLookatRotation (Math|Vector|MakeVector (.x _returnvalue) (.y _returnvalue) 0.0) (Math|Vector|MakeVector (.x _returnvalue_2) (.y _returnvalue_2) 0.0)))
  (AI|Components|Blackboard|SetValueasBool (AI|GetBlackboard (AI|GetAIController self)) (Utilities|Name|MakeLiteralName "CanMove") false)
  (Utilities|FlowControl|Delay 0.2)
  (bind _returnvalue_3 (Animation|Montage|MontagePlay (Components|SkeletalMesh|GetAnimInstance (Variables|Character|GetMesh)) "/Game/Mesh/NPCs/Anims/360_attack_Montage.360_attack_Montage" 1.0 "MontageLength" 0.0 true))
  (Utilities|FlowControl|Sequence
    (:then_0
      (bind (_direction _slashanticipationalpha _slashanticipation _slashfloat) (Timeline|Slash PlayFromStart)
        (:Update
          (Rendering|Material|SetScalarParameterValueonMaterials _slash02 "SlashAnticipationAlpha" _slashanticipationalpha)
          (Rendering|Material|SetScalarParameterValueonMaterials _slash02 "SlashAnticipation" _slashanticipation)
          (Rendering|Material|SetScalarParameterValueonMaterials _slash02 "Slash" _slashfloat))))
    (:then_1
      (Utilities|FlowControl|Delay (+ _returnvalue_3 0.2))
      (AI|Components|Blackboard|SetValueasBool (AI|GetBlackboard (AI|GetAIController self)) (Utilities|Name|MakeLiteralName "CanMove") true)
      (Variables|/Script/Engine.CharacterMovementComponent|SetbOrientRotationToMovement (Variables|Character|GetCharacterMovement) true))))

(event EventOnEndOfSplineReached
  (bind _iteminstance (Variables|Default|GetItemInstance))
  (Utilities|IsValid _iteminstance
    (:Is%20Valid
      (Actor|DestroyActor _iteminstance))
    (:Is%20Not%20Valid
      _))
  (Actor|DestroyActor))

(event EventBeginPlay
  (|CallParentFunction)
  (Transformation|AttachComponentToComponent (Variables|Default|GetCube) (Variables|Character|GetMesh) "PapyHand" "SnapToTarget" "SnapToTarget" "SnapToTarget" true)
  (Utilities|Time|SetTimerbyEvent (delegate Custom|MakePause) (Math|Random|RandomFloatinRange 5.0 15.0)))

(fn ConstructionScript
  (|CallParentFunction))

(fn GetPatrolRoute
  (return 0))