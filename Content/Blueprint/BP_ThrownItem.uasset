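; BP_ThrownItem is a thrown item actor that flies in an arc to a target, then updates the monkey's score and destroys itself.
; BeginPlay lifts the path midpoint by the throw height and picks a random spin.
; Tick moves it along a quadratic Bezier curve over the throw time while interpolating rotation.
; On arrival it adds the monkey's TotalPoints to itself, doubling the total.
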(event EventTick
  (params (DeltaSeconds :type Float%20%28single-precision%29))
  (bind _bp_monkey (CallFunction|GetMonkey))
  (Variables|Default|SetcurrentMovingTime (+ DeltaSeconds (Variables|Default|GetcurrentMovingTime)))
  (Variables|Default|SetnormalizedProgress (Math|Float|Clamp(Float) (/ (Variables|Default|GetcurrentMovingTime) (Variables|Default|GettotalThrowTime))))
  (Variables|Default|SetOneMinusT (- 1.0 (Variables|Default|GetnormalizedProgress)))
  (Transformation|SetActorLocation (+ (* (Variables|Default|GetStartPos) (Math|Float|Square (Variables|Default|GetOneMinusT))) (* (* 2.0 (Variables|Default|GetOneMinusT) (Variables|Default|GetnormalizedProgress)) (Variables|Default|Getmidpoint)) (* (Math|Float|Square (Variables|Default|GetnormalizedProgress)) (Variables|Default|GetTargetPos))) false false)
  (Transformation|SetActorRotation (Math|Rotator|MakeRotator (.x (Math|Vector|Lerp(Vector) "0, 0, 0" (Variables|Default|GetRotation) (Variables|Default|GetnormalizedProgress))) (.y (Math|Vector|Lerp(Vector) "0, 0, 0" (Variables|Default|GetRotation) (Variables|Default|GetnormalizedProgress))) (.z (Math|Vector|Lerp(Vector) "0, 0, 0" (Variables|Default|GetRotation) (Variables|Default|GetnormalizedProgress)))))
  (if (== (Variables|Default|GetnormalizedProgress) 1.0)
    (Variables|/Game/Blueprint/BP_Monkey.BP_Monkey_C|SetTotalPoints _bp_monkey (+ (Variables|/Game/Blueprint/BP_Monkey.BP_Monkey_C|GetTotalPoints _bp_monkey) (Variables|/Game/Blueprint/BP_Monkey.BP_Monkey_C|GetTotalPoints _bp_monkey)))
    (Actor|DestroyActor)))

(event EventBeginPlay
  (Variables|Default|Setmidpoint (+ (/ (+ (Variables|Default|GetStartPos) (Variables|Default|GetTargetPos)) 2.0) (Math|Vector|MakeVector 0.0 0.0 (Variables|Default|GetthrowHeight))))
  (Variables|Default|SetRotation (Math|Vector|MakeVector (Math|Random|RandomFloatinRange 2e+02 7.2e+02) (Math|Random|RandomFloatinRange 2e+02 7.2e+02) (Math|Random|RandomFloatinRange 2e+02 7.2e+02))))

(fn ConstructionScript)