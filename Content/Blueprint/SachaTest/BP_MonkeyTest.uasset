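; Test monkey player character that walks and climbs on slopes, leaving footprint decals.
; Enhanced Input moves it along world axes rotated 45 degrees.
; Each tick, a sphere trace's surface normal drives curve-table walk speed and a climbing flag for the AnimBP, which turns the capsule toward the surface and toggles physics below the shoulder bones.
; Looping timers trace under each foot to spawn fading, surface-aligned decals while moving.
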(event Custom|CheckgroundFrontLeft
  (bind _leftfootcollider (Variables|Default|GetLeftFootCollider))
  (bind _returnvalue (Transformation|GetWorldLocation _leftfootcollider))
  (bind _outhit (Collision|LineTraceByChannel _returnvalue (+ _returnvalue (* (Math|Vector|NegateVector (Transformation|GetActorUpVector)) 1e+02)) "TraceTypeQuery1" false 0 "None"))
  (if (>= (Math|Vector|VectorLength (Variables|/Script/Engine.MovementComponent|GetVelocity (Variables|Character|GetCharacterMovement))) 1e+02)
    (if (<= (.Distance (Collision|BreakHitResult _outhit)) (Variables|Default|GetMaxStepheight))
      _
      (else
        (Utilities|FlowControl|DoOnce false ; enters at Reset
          (:Completed
            _))))
    (bind _returnvalue_2 (Rendering|Decal|SpawnDecalatLocation "/Game/Blueprint/SachaTest/FootDecalLeft.FootDecalLeft" "5.000000,5.000000,5.000000" (.ImpactPoint (Collision|BreakHitResult _outhit)) (Math|Rotator|MakeRotator 0.0 (.pitch (Math|Conversions|RotationFromXVector (Math|Vector|NegateVector (.Normal (Collision|BreakHitResult _outhit))))) (- (.yaw (Transformation|GetSocketRotation (Variables|Character|GetMesh) "L_Foot")) 9e+01)) 5.0))
    (Rendering|Components|Decal|SetFadeOut _returnvalue_2 2.0 3.0 true)))

(event Custom|CheckGroundFrontRight
  (bind _rightfootcollider (Variables|Default|GetRightFootCollider))
  (bind _returnvalue (Transformation|GetWorldLocation _rightfootcollider))
  (bind _outhit (Collision|LineTraceByChannel _returnvalue (+ _returnvalue (* (Math|Vector|NegateVector (Transformation|GetActorUpVector)) 1e+02)) "TraceTypeQuery1" false 0 "None"))
  (if (>= (Math|Vector|VectorLength (Variables|/Script/Engine.MovementComponent|GetVelocity (Variables|Character|GetCharacterMovement))) 1e+02)
    (if (<= (.Distance (Collision|BreakHitResult _outhit)) (Variables|Default|GetMaxStepheight))
      _
      (else
        (Utilities|FlowControl|DoOnce false ; enters at Reset
          (:Completed
            _))))
    (bind _returnvalue_2 (Rendering|Decal|SpawnDecalatLocation "/Game/Blueprint/SachaTest/FootDecalRight.FootDecalRight" "5.000000,5.000000,5.000000" (.ImpactPoint (Collision|BreakHitResult _outhit)) (Math|Rotator|MakeRotator 0.0 (.pitch (Math|Conversions|RotationFromXVector (Math|Vector|NegateVector (.Normal (Collision|BreakHitResult _outhit))))) (- (.yaw (Transformation|GetSocketRotation (Variables|Character|GetMesh) "R_Foot")) 9e+01)) 7.0))
    (Rendering|Components|Decal|SetFadeOut _returnvalue_2 2.0 3.0 true)))

(event Input|EnhancedActionEvents|EnhancedInputActionIA_Move
  (params (ActionValue :type Vector%202D%20Structure) (ElapsedSeconds :type Float%20%28double-precision%29) (TriggeredSeconds :type Float%20%28double-precision%29) (InputAction :type Input%20Action%20Object%20Reference :default "/Game/Blueprint/Inputs/IA_Move.IA_Move"))
  (bind (_right _forward) (CallFunction|GetMovementAxis))
  ;[0 0 0] Movement
  (Pawn|Input|AddMovementInput _right (.x ActionValue) false)
  (Pawn|Input|AddMovementInput _forward (.y ActionValue) false)
  (Rendering|Debug|DrawDebugArrow "0, 0, 0" "0, 0, 0" 0.0 "(R=1.000000,G=0.000000,B=0.702046,A=1.000000)" 0.03 1.0))

(event EventTick
  (params (DeltaSeconds :type Float%20%28single-precision%29))
  (Utilities|FlowControl|Sequence
    (:then_1
      (CallFunction|SetSpeed)
      (CallFunction|OrienttoMovement))
    (:then_2
      (Development|PrintString (Utilities|String|Append "Slope : " (Utilities|String|ToString(Float) (Variables|Default|GetCurrentSlope))) true true "(R=0.000000,G=0.660000,B=1.000000,A=1.000000)" 2.0 "slope")
      (Development|PrintString (Utilities|String|Append "IsClimbing : " (Utilities|String|ToString(Boolean) (Variables|Default|GetbIsCimbing))) true true "(R=0.000000,G=0.660000,B=1.000000,A=1.000000)" 2.0 "isClimbing"))))

(event EventBeginPlay
  (Utilities|FlowControl|Sequence
    (:then_0
      ;[0 0 0] Inputs
      (Input|AddMappingContext (PlayerController|LocalPlayerSubsystems|GetEnhancedInputLocalPlayerSubsystem (Game|GetPlayerController 0)) "/Game/Blueprint/Inputs/IMC_Default.IMC_Default" 0 "(bIgnoreAllPressedKeysUntilRelease=True,bForceImmediately=False,bNotifyUserSettings=False)"))
    (:then_1
      (bind _asabp_monkey_stand (Utilities|Casting|CastToABP_MonkeyStand (Components|SkeletalMesh|GetAnimInstance (Variables|Character|GetMesh))))
      (Variables|Default|SetABP _asabp_monkey_stand))
    (:then_2
      (Utilities|Time|SetTimerbyEvent (delegate Custom|CheckgroundFrontLeft) 0.2 true)
      (Utilities|Time|SetTimerbyEvent (delegate Custom|CheckGroundFrontRight) 0.2 true))))

(fn ConstructionScript)

(fn GetMovementAxis
  (return (Math|Vector|Normalize (Math|Vector|RotateVector (Class|KismetMathLibrary|VectorRight) "0.000000,45.000000,0.000000")) (Math|Vector|Normalize (Math|Vector|RotateVector (Class|KismetMathLibrary|VectorForward) "0.000000,45.000000,0.000000"))))

(fn SetSpeed
  (bind _returnvalue (Transformation|GetActorForwardVector))
  (bind _returnvalue_2 (Transformation|GetActorLocation))
  (bind _returnvalue_3 (* _returnvalue ""))
  (bind _returnvalue_4 (+ _returnvalue_2 _returnvalue_3))
  (bind _outhit (Collision|SphereTraceByChannel _returnvalue_4 _returnvalue_4 5e+01 "TraceTypeQuery1" false 0 "None"))
  (if (.bBlockingHit (Collision|BreakHitResult _outhit))
    (Variables|Default|SetClosestNormal (.ImpactNormal (Collision|BreakHitResult _outhit)))
    (bind _outxy (DataTable|EvaluateCurveTableRow "/Game/Blueprint/PlayerCurveTable.PlayerCurveTable" "Speed" (Math|Float|Absolute(Float) (Math|Vector|DotProduct (.ImpactNormal (Collision|BreakHitResult _outhit)) (Math|Vector|VectorUp))))
      (:RowFound
        (Variables|/Script/Engine.CharacterMovementComponent|SetMaxWalkSpeed (Variables|Character|GetCharacterMovement) _outxy)
        (Development|PrintString (Utilities|String|Append "Speed" (Utilities|String|ToString(Float) _outxy)) true true "(R=0.000000,G=0.660000,B=1.000000,A=1.000000)" 0.16 "c")
        (bind _output_get (Variables|Default|SetCurrentSlope (Class|KismetMathLibrary|DegAcos (Math|Vector|DotProduct (.ImpactNormal (Collision|BreakHitResult _outhit)) (Math|Vector|VectorUp)))))
        (bind _output_get_2 (Variables|Default|SetbIsCimbing (> _output_get (Variables|Default|GetWalkingSlopeMax))))
        (Variables|/Game/Meshes/Monkey/ABP_MonkeyStand.ABP_MonkeyStand_C|SetbIsClimbing (Variables|Default|GetABP) _output_get_2)))))

(fn OrienttoMovement
  (bind _biscimbing (Variables|Default|GetbIsCimbing))
  (bind _returnvalue (not _biscimbing))
  (Class|SkeletalMeshComponent|SetAllBodiesBelowSimulatePhysics (Variables|Character|GetMesh) (Utilities|Name|MakeLiteralName "L_Soulder") _returnvalue false)
  (Class|SkeletalMeshComponent|SetAllBodiesBelowSimulatePhysics (Variables|Character|GetMesh) (Utilities|Name|MakeLiteralName "R_Soulder") _returnvalue false)
  (if (Variables|Default|GetbIsCimbing)
    (Transformation|SetRelativeRotation (Variables|Collision|GetCapsuleComponent) (Math|Rotator|MakeRotationfromAxes (Math|Vector|NegateVector (Variables|Default|GetClosestNormal)) "0, 0, 0" "0, 0, 0") false false)))