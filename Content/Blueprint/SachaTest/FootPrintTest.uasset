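; Test Blueprint that spawns footprint decals where a foot collider meets the ground.
; A timer set on BeginPlay calls a check that line traces from FootCollider along the actor's down vector, with debug drawing on.
; A hit within MaxStepHeight spawns one decal, pitched to the surface normal and yawed from the Cube's socket.
; A DoOnce limits this to one print per step, resetting when the distance exceeds that height.
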(event Custom|CheckgroundFrontRight
  (bind _footcollider (Variables|Default|GetFootCollider))
  (bind _returnvalue (Transformation|GetWorldLocation _footcollider))
  (bind _outhit (Collision|LineTraceByChannel _returnvalue (+ _returnvalue (* (Math|Vector|NegateVector (Transformation|GetActorUpVector)) 1e+02)) "TraceTypeQuery1" false 0 "ForDuration"))
  (if (<= (.Distance (Collision|BreakHitResult _outhit)) (Variables|Default|GetMaxStepHeight))
    (Utilities|FlowControl|DoOnce false :!label _label
      (:Completed
        (Rendering|Decal|SpawnDecalatLocation 0 "10.000000,10.000000,10.000000" (.ImpactPoint (Collision|BreakHitResult _outhit)) (Math|Rotator|MakeRotator 0.0 (.pitch (Math|Conversions|RotationFromXVector (Math|Vector|NegateVector (.Normal (Collision|BreakHitResult _outhit))))) (- (.yaw (Transformation|GetSocketRotation (Variables|Default|GetCube) "cube")) 9e+01)) 0.0)))
    (else
      (goto _label Reset))))

(event EventBeginPlay
  (Utilities|Time|SetTimerbyEvent (delegate Custom|CheckgroundFrontRight) 0.0))

(event Collision|EventActorBeginOverlap
  (params (OtherActor :type Actor%20Object%20Reference)))

(event EventTick
  (params (DeltaSeconds :type Float%20%28single-precision%29)))

(fn ConstructionScript)