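; Spawner actor that periodically creates enemy characters at its own transform.
; BeginPlay starts a looping timer at SpawnRate that calls Spawn, which only proceeds while the Monkey's CanSpawnEnemies flag is set.
; Each spawn picks a random class from CharactersList and passes it a random route from AssociatedPatrolRoutes, adjusting for collisions but always spawning.
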(event EventBeginPlay
  (Utilities|Time|SetTimerbyFunctionName 0 "Spawn" (Variables|Default|GetSpawnRate) true))

(fn ConstructionScript)

(fn Spawn
  (if (Variables|/Game/Blueprint/BP_Monkey.BP_Monkey_C|GetCanSpawnEnemies (CallFunction|GetMonkey))
    (Game|SpawnActorfromClass (.OutItem (Utilities|Array|Random (Variables|Default|GetCharactersList))) (Transformation|GetActorTransform) "AdjustIfPossibleButAlwaysSpawn" "MultiplyWithRoot" 0 (.OutItem (Utilities|Array|Random (Variables|Default|GetAssociatedPatrolRoutes))) 0 0)))