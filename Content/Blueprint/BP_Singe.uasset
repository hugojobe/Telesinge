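; BP_Singe is a character Blueprint that gives the player basic movement through Enhanced Input.
; BeginPlay adds the IMC_Default mapping context to player controller 0's input subsystem.
; The IA_Move action feeds its X and Y values along the actor's right and forward vectors directly into CharacterMovement, so movement is relative to the actor's facing.
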(event Input|EnhancedActionEvents|EnhancedInputActionIA_Move
  (params (ActionValue :type Vector%202D%20Structure) (ElapsedSeconds :type Float%20%28double-precision%29) (TriggeredSeconds :type Float%20%28double-precision%29) (InputAction :type Input%20Action%20Object%20Reference :default "/Game/Blueprint/Inputs/IA_Move.IA_Move"))
  (bind _charactermovement (Variables|Character|GetCharacterMovement))
  (Class|PawnMovementComponent|AddInputVector _charactermovement (* (.x ActionValue) (Transformation|GetActorRightVector)) false)
  (Class|PawnMovementComponent|AddInputVector _charactermovement (* (.y ActionValue) (Transformation|GetActorForwardVector)) false))

(event EventBeginPlay
  (Input|AddMappingContext (PlayerController|LocalPlayerSubsystems|GetEnhancedInputLocalPlayerSubsystem (Game|GetPlayerController 0)) "/Game/Blueprint/Inputs/IMC_Default.IMC_Default" 0 "(bIgnoreAllPressedKeysUntilRelease=True,bForceImmediately=False,bNotifyUserSettings=False)"))

(fn ConstructionScript)