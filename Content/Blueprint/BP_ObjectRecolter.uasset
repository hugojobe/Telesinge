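; BP_ObjectRecolter is a collection point that takes items from the monkey's inventory while the monkey stands inside its area box.
; Overlap begin starts a looping timer that calls ThrowItem, and overlap end clears it.
; Each tick of that timer spawns a BP_ThrownItem from the monkey toward the collector with configurable duration and height, copies the first item's mesh and scale, then removes it from the inventory.
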(event OnComponentBeginOverlap(RecolterArealBox)
  (params (OverlappedComponent :type Primitive%20Component%20Object%20Reference) (OtherActor :type Actor%20Object%20Reference) (OtherComp :type Primitive%20Component%20Object%20Reference) (OtherBodyIndex :type Integer) (bFromSweep :type Boolean) (SweepResult :type Hit%20Result%20Structure%20%28by%20ref%29))
  (if (== OtherActor (Variables|Default|GetMonkey))
    (Utilities|Time|SetTimerbyFunctionName 0 "ThrowItem" 0.65 true true)))

(event OnComponentEndOverlap(RecolterArealBox)
  (params (OverlappedComponent :type Primitive%20Component%20Object%20Reference) (OtherActor :type Actor%20Object%20Reference) (OtherComp :type Primitive%20Component%20Object%20Reference) (OtherBodyIndex :type Integer))
  (if (== OtherActor (Variables|Default|GetMonkey))
    (Utilities|Time|ClearTimerbyFunctionName 0 "ThrowItem")))

(event EventBeginPlay
  (Variables|Default|SetMonkey (CallFunction|GetMonkey)))

(fn ConstructionScript)

(fn ThrowItem
  (bind _monkey (Variables|Default|GetMonkey))
  (bind _monkey_2 (Variables|Default|GetMonkey))
  (bind _returnvalue (Transformation|GetActorLocation _monkey))
  (bind _inventorycomponent (Variables|/Game/Blueprint/BP_Monkey.BP_Monkey_C|GetInventoryComponent _monkey_2))
  (bind _items (Variables|/Game/UI/inventory/Bp_inventorycomponent.Bp_inventorycomponent_C|GetItems _inventorycomponent))
  (bind _output (Utilities|Array|Get(acopy) _items))
  (bind (_name _stackable _quantity _thumbnail _mesh _itemplacement _meshscale) (Utilities|Struct|BreakS_Itemstructure _output))
  (if (> (Utilities|Array|Length _items) 0)
    (bind _returnvalue_2 (Game|SpawnActorfromClass "/Game/Blueprint/BP_ThrownItem.BP_ThrownItem_C" (Math|Transform|MakeTransform _returnvalue "0, 0, 0" "1.000000,1.000000,1.000000") "Undefined" "MultiplyWithRoot" 0 _returnvalue (Transformation|GetActorLocation) (Variables|Default|GetItemThrowDuration) (Variables|Default|GetItemThrowHeight) 0))
    (Components|StaticMesh|SetStaticMesh (Variables|/Game/Blueprint/BP_ThrownItem.BP_ThrownItem_C|GetStaticMesh _returnvalue_2) _mesh)
    (Transformation|SetRelativeScale3D (Variables|/Game/Blueprint/BP_ThrownItem.BP_ThrownItem_C|GetStaticMesh _returnvalue_2) _meshscale)
    (Utilities|Array|RemoveIndex (Variables|/Game/UI/inventory/Bp_inventorycomponent.Bp_inventorycomponent_C|GetItems (Variables|/Game/Blueprint/BP_Monkey.BP_Monkey_C|GetInventoryComponent (Variables|Default|GetMonkey))))))