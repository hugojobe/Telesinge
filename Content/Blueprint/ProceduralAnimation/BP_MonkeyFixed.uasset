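; Monkey player character with slope-aware climbing and a hold-to-steal interaction, linked to ABP_MonkeyFixed.
; Enhanced Input moves it along world axes rotated 45 degrees.
; Each tick, a sphere trace reads the surface normal to set walk speed from a curve table, pass climbing state to the AnimBP and turn the capsule toward steep surfaces.
; Interact drives FOV zoom timelines with debug steal progress, gated by a climbing tag.
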(event Input|EnhancedActionEvents|EnhancedInputActionIA_Move
  (params (ActionValue :type Vector%202D%20Structure) (ElapsedSeconds :type Float%20%28double-precision%29) (TriggeredSeconds :type Float%20%28double-precision%29) (InputAction :type Input%20Action%20Object%20Reference :default "/Game/Blueprint/Inputs/IA_Move.IA_Move"))
  (bind (_right _forward) (CallFunction|GetMovementAxis))
  ;[0 0 0] Movement
  (Pawn|Input|AddMovementInput _right (.x ActionValue) false)
  (Pawn|Input|AddMovementInput _forward (.y ActionValue) false)
  (Rendering|Debug|DrawDebugArrow "0, 0, 0" "0, 0, 0" 0.0 "(R=1.000000,G=0.000000,B=0.702046,A=1.000000)" 0.03 1.0))

(event Input|EnhancedActionEvents|EnhancedInputActionIA_Interact
  (params (ActionValue :type Boolean) (ElapsedSeconds :type Float%20%28double-precision%29) (TriggeredSeconds :type Float%20%28double-precision%29) (InputAction :type Input%20Action%20Object%20Reference :default "/Game/Blueprint/Inputs/IA_Interact.IA_Interact"))
  (bind _self self)
  (bind _returnvalue (Actor|ActorHasTag _self "Locomotion.Climbing"))
  (bind _returnvalue_2 (not _returnvalue))
  (:Triggered
    (if _returnvalue_2
      (Utilities|FlowControl|DoOnce false :!label _label
        (:Completed
          (bind _outalpha (Timeline|OutZoomTimeline PlayFromStart)
            (:Update
              (Camera|SetFieldOfView (Variables|Default|GetCamera) (Math|Float|Lerp (Variables|Default|GetCamZoomFOV) (Variables|Default|GetCamBaseFOV) _outalpha)))
            (:Finished
              (bind (_direction _alpha) (Timeline|Steal%20Zoom%20Timeline SetNewTime)
                (:Update
                  (Camera|SetFieldOfView (Variables|Default|GetCamera) (Math|Float|Lerp (Variables|Default|GetCamBaseFOV) (Variables|Default|GetCamZoomFOV) _alpha))
                  (if (Utilities|Enum|Equal(Enum) _direction "Forward")
                    (Development|PrintString (Utilities|String|Append "Stealing: " (Utilities|String|ToString(Integer) (Math|Float|Round (* _alpha 1e+02))) "%") true true "(R=1.000000,G=0.000000,B=0.230923,A=1.000000)" 0.02 "bguh"))))))))))
  (:Started
    (if _returnvalue_2
      (Utilities|FlowControl|Sequence
        (:then_0
          (goto _label Reset))
        (:then_1
          (Components|Timeline|SetPlayRate (Variables|Default|GetSteal%20Zoom%20Timeline) 1.0)
          (Timeline|Steal%20Zoom%20Timeline Play)))))
  (:Canceled
    (if _returnvalue_2
      (Components|Timeline|SetPlayRate (Variables|Default|GetSteal%20Zoom%20Timeline) 9.0)
      (Timeline|Steal%20Zoom%20Timeline Reverse))))

(event EventBeginPlay
  (Utilities|FlowControl|Sequence
    (:then_0
      ;[0 0 0] Inputs
      (Input|AddMappingContext (PlayerController|LocalPlayerSubsystems|GetEnhancedInputLocalPlayerSubsystem (Game|GetPlayerController 0)) "/Game/Blueprint/Inputs/IMC_Default.IMC_Default" 0 "(bIgnoreAllPressedKeysUntilRelease=True,bForceImmediately=False,bNotifyUserSettings=False)"))
    (:then_1
      (bind _asabp_monkey_fixed (Utilities|Casting|CastToABP_MonkeyFixed (Components|SkeletalMesh|GetAnimInstance (Variables|Character|GetMesh))))
      (Variables|Default|SetABP _asabp_monkey_fixed))))

(event EventTick
  (params (DeltaSeconds :type Float%20%28single-precision%29))
  (Utilities|FlowControl|Sequence
    (:then_1
      (CallFunction|SetSpeed)
      (CallFunction|OrienttoMovement))
    (:then_2
      ;[0.0999 0.016 0.016] DEBUG
      (Development|PrintString (Utilities|String|Append "Slope : " (Utilities|String|ToString(Float) (Variables|Default|GetCurrentSlope))) true true "(R=0.000000,G=0.660000,B=1.000000,A=1.000000)" 2.0 "slope")
      (Development|PrintString (Utilities|String|Append "IsClimbing : " (Utilities|String|ToString(Boolean) (Variables|Default|GetbIsCimbing))) true true "(R=0.000000,G=0.660000,B=1.000000,A=1.000000)" 2.0 "isClimbing"))))

(fn ConstructionScript)

(fn GetMovementAxis
  (return (Math|Vector|Normalize (Math|Vector|RotateVector (Class|KismetMathLibrary|VectorRight) "0.000000,45.000000,0.000000")) (Math|Vector|Normalize (Math|Vector|RotateVector (Class|KismetMathLibrary|VectorForward) "0.000000,45.000000,0.000000"))))

(fn SetSpeed
  (bind _returnvalue (Transformation|GetActorForwardVector))
  (bind _returnvalue_2 (Transformation|GetActorLocation))
  (bind _returnvalue_3 (* _returnvalue ""))
  (bind _returnvalue_4 (+ _returnvalue_2 _returnvalue_3))
  (bind _outhit (Collision|SphereTraceByChannel _returnvalue_4 _returnvalue_4 5e+01 "TraceTypeQuery1" false 0 "None"))
  (if (.bBlockingHit (Collision|BreakHitResult _outhit))
    (Variables|Default|SetClosestNormal (.ImpactNormal (Collision|BreakHitResult _outhit)))
    (bind _outxy (DataTable|EvaluateCurveTableRow "/Game/Blueprint/PlayerCurveTable.PlayerCurveTable" "Speed" (Math|Float|Absolute(Float) (Math|Vector|DotProduct (.ImpactNormal (Collision|BreakHitResult _outhit)) (Math|Vector|VectorUp))))
      (:RowFound
        (Variables|/Script/Engine.CharacterMovementComponent|SetMaxWalkSpeed (Variables|Character|GetCharacterMovement) _outxy)
        (Development|PrintString (Utilities|String|Append "Speed" (Utilities|String|ToString(Float) _outxy)) true true "(R=0.000000,G=0.660000,B=1.000000,A=1.000000)" 0.16 "c")
        (bind _output_get (Variables|Default|SetCurrentSlope (Class|KismetMathLibrary|DegAcos (Math|Vector|DotProduct (.ImpactNormal (Collision|BreakHitResult _outhit)) (Math|Vector|VectorUp)))))
        (bind _output_get_2 (Variables|Default|SetbIsCimbing (> _output_get (Variables|Default|GetWalkingSlopeMax))))
        (Variables|/Game/Blueprint/ProceduralAnimation/ABP_MonkeyFixed.ABP_MonkeyFixed_C|SetbIsClimbing (Variables|Default|GetABP) _output_get_2)
        (Variables|/Game/Blueprint/ProceduralAnimation/ABP_MonkeyFixed.ABP_MonkeyFixed_C|SetclosestSurfaceNormal (Variables|Default|GetABP) (Variables|Default|GetClosestNormal))))))

(fn OrienttoMovement
  ;[0 0 0] For BIPED
  (Class|SkeletalMeshComponent|SetAllBodiesBelowSimulatePhysics (Variables|Character|GetMesh) (Utilities|Name|MakeLiteralName "L_Soulder") false false)
  (Class|SkeletalMeshComponent|SetAllBodiesBelowSimulatePhysics (Variables|Character|GetMesh) (Utilities|Name|MakeLiteralName "R_Soulder") false false)
  (if (Variables|Default|GetbIsCimbing)
    (Transformation|SetRelativeRotation (Variables|Collision|GetCapsuleComponent) (Math|Rotator|MakeRotationfromAxes (Math|Vector|NegateVector (Variables|Default|GetClosestNormal)) "0, 0, 0" "0, 0, 0") false false)))