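; Chest inventory component that creates a WB_Coffre widget on BeginPlay and stores it for later use.
; The remaining logic is disconnected and never runs.
; It holds a sphere-trace pickup that stacks Bp_item2 items up to 64 or fills empty slots, then refreshes the widget and destroys the item.
; Also unwired are a widget visibility toggle with cursor and input-mode switching, and an Items resize to 40 slots.
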(event EventBeginPlay
  (bind _returnvalue (UserInterface|CreateWidget "/Game/UI2/Chest/WB_Coffre.WB_Coffre_C"))
  (Variables|Default|SetCOffreinventorywidget _returnvalue))

(event EventTick
  (params (DeltaSeconds :type Float%20%28single-precision%29)))

(event Input|KeyboardEvents|C
  (params (Key :type Key%20Structure)))

(event Input|KeyboardEvents|V
  (params (Key :type Key%20Structure)))