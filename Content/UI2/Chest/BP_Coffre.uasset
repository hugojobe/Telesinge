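; BP_Coffre is a chest actor that shows its WB_Coffre inventory widget while its trigger box is overlapped.
; BeginPlay creates the widget hidden in the viewport and caches the player's BP_Monkey reference; box begin and end overlap toggle visibility, with no check on the overlapping actor.
; Deposit, widget refresh of fame and cosmetic items, and input-mode restore nodes exist but are unconnected, and the Overlap function is empty.
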(event OnComponentBeginOverlap(Box)
  (params (OverlappedComponent :type Primitive%20Component%20Object%20Reference) (OtherActor :type Actor%20Object%20Reference) (OtherComp :type Primitive%20Component%20Object%20Reference) (OtherBodyIndex :type Integer) (bFromSweep :type Boolean) (SweepResult :type Hit%20Result%20Structure%20%28by%20ref%29))
  (Widget|SetVisibility (Variables|Default|GetWidget) "Visible"))

(event OnComponentEndOverlap(Box)
  (params (OverlappedComponent :type Primitive%20Component%20Object%20Reference) (OtherActor :type Actor%20Object%20Reference) (OtherComp :type Primitive%20Component%20Object%20Reference) (OtherBodyIndex :type Integer))
  (Widget|SetVisibility (Variables|Default|GetWidget) "Hidden"))

(event EventBeginPlay
  (bind _returnvalue (UserInterface|CreateWidget "/Game/UI2/Chest/WB_Coffre.WB_Coffre_C"))
  (bind _output_get (Variables|Default|SetWidget _returnvalue))
  (UserInterface|Viewport|AddtoViewport _output_get 0)
  (Widget|SetVisibility (Variables|Default|GetWidget) "Hidden")
  (bind _asbp_monkey (Utilities|Casting|CastToBP_Monkey (Game|GetPlayerCharacter 0)))
  (Variables|Default|SetPersoReference _asbp_monkey))

(fn ConstructionScript)

(fn Overlap)